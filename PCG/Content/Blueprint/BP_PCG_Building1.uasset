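; Procedural building actor that drives a PCG graph to lay out a modular building of floors, walls, corners and a separately scaled first wall.
; The construction script optionally randomizes floor count, rows and columns, then derives building height and footprint from wall dimensions.
; It pushes the resulting offsets, grid extents and mesh-fitting scale ratios as vector parameters to the PCG component's graph instance.
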(event EventBeginPlay)

(event Collision|EventActorBeginOverlap
  (params (OtherActor :type Actor%20Object%20Reference)))

(event EventTick
  (params (DeltaSeconds :type Float%20%28single-precision%29)))

(fn ConstructionScript
  (bind _wallwidth (Variables|Default|GetWallWidth))
  (bind _floorsize (Variables|Default|GetFloorSize))
  (bind _wallthickness (Variables|Default|GetWallThickness))
  (bind _firstwallcornersize (Variables|Default|GetFirstWallCornerSize))
  (bind _wallwidth_2 (Variables|Default|GetWallWidth))
  (bind _returnvalue (/ _wallwidth _floorsize))
  (bind _returnvalue_2 (/ _wallwidth_2 2.0))
  (Utilities|FlowControl|Sequence
    (:then_0
      ;[0.15 0.15 0.15 0.5] Random Setting
      (if (Variables|Default|GetUseRandomBuilding)
        (Variables|Default|SetNumberOfFloors (Math|Random|RandomIntegerinRange 3 45))
        (Variables|Default|SetBuildingRow (Math|Random|RandomIntegerinRange 3 10))
        (Variables|Default|SetBuildingColumn (Math|Random|RandomIntegerinRange 3 10))))
    (:then_1
      (LocalVariables|SetGraphInstancePCG (Variables|/Script/PCG.PCGComponent|GetGraphInstance (Variables|Default|GetPCG)))
      (LocalVariables|SetBuildingHeight (* (Variables|Default|GetWallHeight) (Variables|Default|GetNumberOfFloors)))
      (LocalVariables|SetBuildingSize (Math|Vector2D|MakeVector2D (* (Variables|Default|GetWallWidth) (Variables|Default|GetBuildingRow)) (* (Variables|Default|GetWallWidth) (Variables|Default|GetBuildingColumn))))
      (bind _output_get (LocalVariables|SetHalfWallWidth (/ (Variables|Default|GetWallWidth) 2.0)))
      (LocalVariables|SetHalfWallWidthNegate (* _output_get -1.0)))
    (:then_2
      (Effects|Components|ParticleSystem|SetVectorParameter (LocalVariables|GetGraphInstancePCG) "FloorScale" (Math|Vector|MakeVector _returnvalue _returnvalue 1.0))
      (Effects|Components|ParticleSystem|SetVectorParameter (LocalVariables|GetGraphInstancePCG) "FloorOffset" (Math|Vector|MakeVector (* _returnvalue_2 -1.0) _returnvalue_2 0.0))
      ;[0.15 0.15 0.15 0.5] Right
      (Effects|Components|ParticleSystem|SetVectorParameter (LocalVariables|GetGraphInstancePCG) "WallOffset1" (Math|Vector|MakeVector 0.0 (/ (Variables|Default|GetWallWidth) 2.0) 0.0))
      ;[0.15 0.15 0.15 0.5] Left
      (Effects|Components|ParticleSystem|SetVectorParameter (LocalVariables|GetGraphInstancePCG) "WallOffset2" (Math|Vector|MakeVector 0.0 (* (/ (Variables|Default|GetWallWidth) 2.0) -1.0) 0.0))
      ;[0.15 0.15 0.15 0.5] Forward
      (Effects|Components|ParticleSystem|SetVectorParameter (LocalVariables|GetGraphInstancePCG) "WallOffset3" (Math|Vector|MakeVector (/ (Variables|Default|GetWallWidth) 2.0) 0.0 0.0))
      ;[0.15 0.15 0.15 0.5] Backward
      (Effects|Components|ParticleSystem|SetVectorParameter (LocalVariables|GetGraphInstancePCG) "WallOffset4" (Math|Vector|MakeVector (* (/ (Variables|Default|GetWallWidth) 2.0) -1.0) 0.0 0.0))
      ;[0.15 0.15 0.15 0.5] Wall Offset Adjustment
      (Effects|Components|ParticleSystem|SetVectorParameter (LocalVariables|GetGraphInstancePCG) "WallOffsetAdjustment" (Math|Vector|MakeVector (* (/ (Variables|Default|GetWallWidth) 2.0) -1.0) (Variables|Default|GetWallThickness) 0.0)))
    (:then_3
      (Effects|Components|ParticleSystem|SetVectorParameter (LocalVariables|GetGraphInstancePCG) "HighestWallOffset" (Math|Vector|MakeVector 0.0 0.0 (- (LocalVariables|GetBuildingHeight) (Variables|Default|GetWallHeight))))
      (Effects|Components|ParticleSystem|SetVectorParameter (LocalVariables|GetGraphInstancePCG) "WallGridExtents" (Math|Vector|MakeVector (/ (.x (LocalVariables|GetBuildingSize)) 2.0) (/ (.y (LocalVariables|GetBuildingSize)) 2.0) 0.0)))
    (:then_4
      ;[0.15 0.15 0.15 0.5] Corner
      (Effects|Components|ParticleSystem|SetVectorParameter (LocalVariables|GetGraphInstancePCG) "CornerOffset1" (Math|Vector|MakeVector (LocalVariables|GetHalfWallWidthNegate) (LocalVariables|GetHalfWallWidth) 0.0))
      (Effects|Components|ParticleSystem|SetVectorParameter (LocalVariables|GetGraphInstancePCG) "CornerOffset2" (Math|Vector|MakeVector (LocalVariables|GetHalfWallWidthNegate) (LocalVariables|GetHalfWallWidthNegate) 0.0))
      (Effects|Components|ParticleSystem|SetVectorParameter (LocalVariables|GetGraphInstancePCG) "CornerOffset3" (Math|Vector|MakeVector (LocalVariables|GetHalfWallWidth) (LocalVariables|GetHalfWallWidthNegate) 0.0))
      (Effects|Components|ParticleSystem|SetVectorParameter (LocalVariables|GetGraphInstancePCG) "CornerOffset4" (Math|Vector|MakeVector (LocalVariables|GetHalfWallWidth) (LocalVariables|GetHalfWallWidth) 0.0))
      (Effects|Components|ParticleSystem|SetVectorParameter (LocalVariables|GetGraphInstancePCG) "CornerOffsetAdjustment" (Math|Vector|MakeVector (* _wallthickness -1.0) _wallthickness 0.0))
      (Effects|Components|ParticleSystem|SetVectorParameter (LocalVariables|GetGraphInstancePCG) "CornerScale" (Math|Vector|MakeVector 1.0 (/ (Variables|Default|GetWallThickness) (Variables|Default|GetCornerThickness)) 1.0)))
    (:then_5
      ;[0.15 0.15 0.15 0.5] First Wall
      (Effects|Components|ParticleSystem|SetVectorParameter (LocalVariables|GetGraphInstancePCG) "FirstWallHeightOffset" (Math|Vector|MakeVector 0.0 0.0 (Variables|Default|GetWallHeight)))
      (Effects|Components|ParticleSystem|SetVectorParameter (LocalVariables|GetGraphInstancePCG) "FirstWallScale" (Math|Vector|MakeVector (/ (Variables|Default|GetWallWidth) (Variables|Default|GetFirstWallWidth)) (/ (Variables|Default|GetWallThickness) (Variables|Default|GetFirstWallThickness)) (/ (Variables|Default|GetWallHeight) (Variables|Default|GetFirstWallHeight))))
      (Effects|Components|ParticleSystem|SetVectorParameter (LocalVariables|GetGraphInstancePCG) "FirstWallCornerScale" (Math|Vector|MakeVector (/ (Variables|Default|GetCornerWidth) (.x _firstwallcornersize)) (/ (Variables|Default|GetWallThickness) (.y _firstwallcornersize)) (/ (Variables|Default|GetCornerHeight) (.z _firstwallcornersize)))))))