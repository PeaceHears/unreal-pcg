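; Spline-based PCG building actor that drives a PCG graph instance from wall, floor and floor-count settings.
; The construction script computes building height from wall height and floor count.
; It then writes vector parameters into the graph: floor scale and offset, four directional wall offsets, an adjustment offset, and a top-floor wall offset.
; Offsets derive from half the wall width, so pieces follow the module size.
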(event EventBeginPlay)

(event Collision|EventActorBeginOverlap
  (params (OtherActor :type Actor%20Object%20Reference)))

(event EventTick
  (params (DeltaSeconds :type Float%20%28single-precision%29)))

(fn ConstructionScript
  (bind _wallwidth (Variables|Default|GetWallWidth))
  (bind _floorsize (Variables|Default|GetFloorSize))
  (bind _wallwidth_2 (Variables|Default|GetWallWidth))
  (bind _returnvalue (/ _wallwidth _floorsize))
  (bind _returnvalue_2 (/ _wallwidth_2 2.0))
  (Utilities|FlowControl|Sequence
    (:then_0
      (LocalVariables|SetGraphInstancePCG (Variables|/Script/PCG.PCGComponent|GetGraphInstance (Variables|Default|GetPCG)))
      (LocalVariables|SetBuildingHeight (* (Variables|Default|GetWallHeight) (Variables|Default|GetNumberOfFloors))))
    (:then_1
      (Effects|Components|ParticleSystem|SetVectorParameter (LocalVariables|GetGraphInstancePCG) "FloorScale" (Math|Vector|MakeVector _returnvalue _returnvalue 1.0))
      (Effects|Components|ParticleSystem|SetVectorParameter (LocalVariables|GetGraphInstancePCG) "FloorOffset" (Math|Vector|MakeVector (* _returnvalue_2 -1.0) _returnvalue_2 0.0))
      ;[0.15 0.15 0.15 0.5] Right
      (Effects|Components|ParticleSystem|SetVectorParameter (LocalVariables|GetGraphInstancePCG) "WallOffset1" (Math|Vector|MakeVector 0.0 (/ (Variables|Default|GetWallWidth) 2.0) 0.0))
      ;[0.15 0.15 0.15 0.5] Left
      (Effects|Components|ParticleSystem|SetVectorParameter (LocalVariables|GetGraphInstancePCG) "WallOffset2" (Math|Vector|MakeVector 0.0 (* (/ (Variables|Default|GetWallWidth) 2.0) -1.0) 0.0))
      ;[0.15 0.15 0.15 0.5] Forward
      (Effects|Components|ParticleSystem|SetVectorParameter (LocalVariables|GetGraphInstancePCG) "WallOffset3" (Math|Vector|MakeVector (/ (Variables|Default|GetWallWidth) 2.0) 0.0 0.0))
      ;[0.15 0.15 0.15 0.5] Backward
      (Effects|Components|ParticleSystem|SetVectorParameter (LocalVariables|GetGraphInstancePCG) "WallOffset4" (Math|Vector|MakeVector (* (/ (Variables|Default|GetWallWidth) 2.0) -1.0) 0.0 0.0))
      ;[0.15 0.15 0.15 0.5] Wall Offset Adjustment
      (Effects|Components|ParticleSystem|SetVectorParameter (LocalVariables|GetGraphInstancePCG) "WallOffsetAdjustment" (Math|Vector|MakeVector (* (/ (Variables|Default|GetWallWidth) 2.0) -1.0) 0.0 0.0)))
    (:then_2
      (Effects|Components|ParticleSystem|SetVectorParameter (LocalVariables|GetGraphInstancePCG) "HighestWallOffset" (Math|Vector|MakeVector 0.0 0.0 (- (LocalVariables|GetBuildingHeight) (Variables|Default|GetWallHeight)))))))